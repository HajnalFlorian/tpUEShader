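; Player Blueprint that handles basic character locomotion, camera look and jumping from player input.
; MoveForward and MoveRight axes add movement input along the forward and right vectors of the full control rotation, so movement follows the view direction.
; Turn and LookUp axes feed controller yaw and pitch, while the Jump action starts and stops the built-in Character jump.
; The construction script is empty.
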(event Input|ActionEvents|InputActionJump
  (params (Key :type Key%20Structure :default "None"))
  ;[1 1 1] Input souris+input barre espace Jump
  (:Pressed
    (Character|Jump))
  (:Released
    (Character|StopJumping)))

(event Input|AxisEvents|InputAxisMoveForward
  (params (AxisValue :type Float%20%28single-precision%29))
  ;[1 1 1] Input clavier deplacement
  (Pawn|Input|AddMovementInput (Math|Vector|GetForwardVector (Pawn|GetControlRotation :!class /Script/Engine.Pawn)) AxisValue false))

(event Input|AxisEvents|InputAxisMoveRight
  (params (AxisValue :type Float%20%28single-precision%29))
  ;[1 1 1] Input clavier deplacement
  (Pawn|Input|AddMovementInput (Math|Vector|GetRightVector (Pawn|GetControlRotation :!class /Script/Engine.Pawn)) AxisValue false))

(event Input|AxisEvents|InputAxisTurn
  (params (AxisValue :type Float%20%28single-precision%29))
  ;[1 1 1] Input souris+input barre espace Jump
  (Pawn|Input|AddControllerYawInput AxisValue))

(event Input|AxisEvents|InputAxisLookUp
  (params (AxisValue :type Float%20%28single-precision%29))
  ;[1 1 1] Input souris+input barre espace Jump
  (Pawn|Input|AddControllerPitchInput AxisValue))

(fn ConstructionScript)